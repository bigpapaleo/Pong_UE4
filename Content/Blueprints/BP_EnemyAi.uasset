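; BP_EnemyAi is an AI opponent whose Cube tracks the BP_Ball actor, like a paddle.
; Each Tick, throttled by TickInterval set at BeginPlay, looks up the ball and stores its Sphere's relative location.
; Move then uses MoveComponentTo over OverTime to slide the Cube's relative Z toward the ball's X, clamped to a fixed range.
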(event Custom|Move
  (Components|MoveComponentTo (Variables|Default|GetCube) (Math|Vector|MakeVector 0.0 0.0 (Math|Float|Clamp(Float) (.x (Variables|Default|GetLocation_Ball)) -3.9e+02 3.9e+02)) "0, 0, 0" false false (Variables|Default|GetOver%20Time) false))

(event EventBeginPlay
  (Actor|Tick|SetActorTickInterval (Variables|Default|GetTick%20Interval)))

(event Collision|EventActorBeginOverlap
  (params (OtherActor :type Actor%20Object%20Reference)))

(event EventTick
  (params (DeltaSeconds :type Float%20%28single-precision%29))
  (bind _returnvalue (Actor|GetActorOfClass "/Game/Blueprints/BP_Ball.BP_Ball_C"))
  (Utilities|IsValid _returnvalue
    (:Is%20Valid
      (Variables|Default|SetLocation_Ball (Variables|/Script/Engine.SceneComponent|GetRelativeLocation (Variables|/Game/Blueprints/BP_Ball.BP_Ball_C|GetSphere _returnvalue)))
      (CallFunction|Move))))

(fn ConstructionScript)