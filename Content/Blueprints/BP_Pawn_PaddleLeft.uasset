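; Left paddle pawn that the player moves along its local Z axis and that also creates the HUD on BeginPlay.
; Each Tick offsets the SMPlayer01 component by a scaled input axis value, without delta-time scaling, so speed depends on frame rate.
; ChangingSpeed sets SpeedMin and SpeedMax, but the clamp that reads them is unconnected, so they do not affect movement.
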(event EventBeginPlay
  (bind _returnvalue (UserInterface|CreateWidget "/Game/UI/Widget_Hud.Widget_Hud_C"))
  (UserInterface|Viewport|AddtoViewport _returnvalue 0))

(event Collision|EventActorBeginOverlap
  (params (OtherActor :type Actor%20Object%20Reference)))

(event EventTick
  (params (DeltaSeconds :type Float%20%28single-precision%29))
  (Transformation|AddLocalOffset (Variables|Default|GetSM_Player01) (Math|Vector|MakeVector 0.0 0.0 (* (Class|Actor|GetInputAxisKeyValue) 1e+01)) false false))

(fn ConstructionScript)

(fn ChangingSpeed
  (params (Speed_Min :type Float%20%28single-precision%29) (Speed_Max :type Float%20%28single-precision%29))
  (Variables|Default|SetSpeed_Min Speed_Min)
  (Variables|Default|SetSpeed_Max Speed_Max))